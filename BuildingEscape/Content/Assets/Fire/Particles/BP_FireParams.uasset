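; BP_FireParams is a fire effect actor that exposes tunable colors for a Niagara particle system.
; Its Construction Script pushes the smoke, fire, and ember start and end color variables into the matching Niagara color parameters.
; Colors are applied at construction, and the event graph holds only disabled stub events with no runtime logic.
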(fn `UserConstructionScript`
  (`FXSystemComponent.SetColorParameter` (`self.Niagara`) "Smoke Color" (`self.Smoke Color`))
  (`FXSystemComponent.SetColorParameter` (`self.Niagara`) "Fire Color" (`self.Fire Color`))
  (`FXSystemComponent.SetColorParameter` (`self.Niagara`) "Start Ember Color" (`self.Ember Start Color`))
  (`FXSystemComponent.SetColorParameter` (`self.Niagara`) "End Ember Color" (`self.Ember End Color`)))